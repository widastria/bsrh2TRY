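; Player character for a 2.5D sprite game, handling Enhanced Input movement, jumping, mouse-aimed attacks and view rotation.
; Movement follows the control yaw and flips the sprite, while jumps and attacks jump to animation nodes.
; Attacks face the sprite toward a cursor line trace hit, with a timed window selecting the second combo swing.
; Timelines turn the control rotation between Left, Forward and Right states, which also set the sprite-flip axis.
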(event `self.ReceiveBeginPlay`
  ;[1 0.714 0.6236] BEGIN PLAY
  (bind _asplayer_controller (cast `PlayerController` (`self.GetController`)))
  (`EnhancedInputSubsystemInterface.AddMappingContext` (pcsubsystem `EnhancedInputLocalPlayerSubsystem` _asplayer_controller) "/Game/Input/IMC_Player.IMC_Player" 0 (struct))
  (set `PlayerController.bShowMouseCursor` true _asplayer_controller))

(event `EnhancedInput|/Game/Input/IA_Move`
  (params (ActionValue :type "Float (double-precision)") (ElapsedSeconds :type "Float (double-precision)") (TriggeredSeconds :type "Float (double-precision)") (InputAction :type "InputAction Object Reference" :default "/Game/Input/IA_Move.IA_Move"))
  (bind (_returnvalue_roll _returnvalue_pitch _returnvalue_yaw) (`KismetMathLibrary.BreakRotator` (`self.GetControlRotation`)))
  (bind _sprite (`self.Sprite`))
  ;[0 0.02997 0.07812] Movement
  (:`Triggered`
    (if (`self.CanMove`)
      (`self.AddMovementInput` (`KismetMathLibrary.GetForwardVector` (`KismetMathLibrary.MakeRotator` 0.0 0.0 _returnvalue_yaw)) ActionValue)
      (if (`self.CanFlipSprite`)
        (`/Engine/EditorBlueprintResources/StandardMacros.IsValid` _sprite
          (:`Is Valid`
            (`SceneComponent.K2_SetRelativeRotation` _sprite (select `bool` (> ActionValue 0.0) :`false` (`KismetMathLibrary.MakeRotator` 0.0 0.0 180.0) :`true` (`KismetMathLibrary.MakeRotator` 0.0)) false false)))))))

(event `EnhancedInput|/Game/Input/IA_Jump`
  (params (ActionValue :type Boolean) (ElapsedSeconds :type "Float (double-precision)") (TriggeredSeconds :type "Float (double-precision)") (InputAction :type "InputAction Object Reference" :default "/Game/Input/IA_Jump.IA_Jump"))
  ;[0 0.02997 0.07812] Movement
  (:`Started`
    (`self.Jump`))
  (:`Canceled`
    (`self.StopJumping`)))

(event `self.OnJumped`
  ;[0 0.02997 0.07812] Movement
  (`PaperZDAnimInstance.JumpToNode` (`PaperZDAnimationComponent.AnimInstance` (`self.AnimationComponent`)) "InAir" "None"))

(event `EnhancedInput|/Game/Input/IA_Attack`
  (params (ActionValue :type Boolean) (ElapsedSeconds :type "Float (double-precision)") (TriggeredSeconds :type "Float (double-precision)") (InputAction :type "InputAction Object Reference" :default "/Game/Input/IA_Attack.IA_Attack"))
  (bind _animinstance (`PaperZDAnimationComponent.AnimInstance` (`self.AnimationComponent`)))
  ;[0.1615 0.03027 0.03027] ATTACK
  (:`Started`
    (if (`self.CanAttack`)
      (set `self.CanMove` true)
      (set `self.CanFlipSprite` false)
      (set `self.CanAttack` false)
      (if (`self.ActivateCombo`)
        (`PaperZDAnimInstance.JumpToNode` _animinstance "AttackSecond" "None")
        (bind _outhit (`self.MouseLineTrace`))
        (`self.FlipSprite` (`.Location` (`GameplayStatics.BreakHitResult` _outhit)))
        (else
          (`PaperZDAnimInstance.JumpToNode` _animinstance "AttackFirst" "None")
          (bind _outhit_2 (`self.MouseLineTrace`))
          (`self.FlipSprite` (`.Location` (`GameplayStatics.BreakHitResult` _outhit_2)))
          (set `self.ActivateCombo` true)
          (`KismetSystemLibrary.K2_SetTimerDelegate` (delegate `CustomEvent`) 1.0))))))

(event `CustomEvent`
  ;[0.1615 0.03027 0.03027] ATTACK
  (set `self.ActivateCombo` false))

(event `EnhancedInput|/Game/Input/IA_Rotate`
  (params (ActionValue :type "Float (double-precision)") (ElapsedSeconds :type "Float (double-precision)") (TriggeredSeconds :type "Float (double-precision)") (InputAction :type "InputAction Object Reference" :default "/Game/Input/IA_Rotate.IA_Rotate"))
  (bind _returnvalue (< ActionValue 0.0))
  ;[0.08725 0.08368 0.1354] Rotation
  (:`Started`
    (if (`self.CanRotatePlayer`)
      (set `self.CanRotatePlayer` false)
      (switch `name` (`self.RotationDirection`)
        (:`Forward`
          (if _returnvalue
            (set `self.RotationDirection` "Right")
            (bind (_direction _rotationtrack) (`Timeline|CharRotationRight` :!label _label)
              (:`Update`
                (`Controller.SetControlRotation` (`self.GetController`) (`KismetMathLibrary.MakeRotator` 0.0 0.0 _rotationtrack)))
              (:`Finished`
                (set `self.CanRotatePlayer` true :!label _label_2)))
            (else
              (set `self.RotationDirection` "Left")
              (bind (_direction_2 _rotationtrack_2) (`Timeline|CharRotationLeft` :!label _label_3)
                (:`Update`
                  (`Controller.SetControlRotation` (`self.GetController`) (`KismetMathLibrary.MakeRotator` 0.0 0.0 _rotationtrack_2)))
                (:`Finished`
                  (goto _label_2))))))
        (:`Right`
          (if _returnvalue
            (goto _label_2)
            (else
              (set `self.RotationDirection` "Forward")
              (goto _label :!via `Reverse`))))
        (:`Left`
          (if _returnvalue
            (set `self.RotationDirection` "Forward")
            (goto _label_3 :!via `Reverse`)
            (else
              (goto _label_2))))))))

(fn `FlipSprite`
  (params (InVec :type "Vector Structure"))
  (bind _returnvalue (> (.x InVec) (.x (`SceneComponent.K2_GetComponentLocation` (`self.CapsuleComponent`)))))
  (switch `name` (`self.RotationDirection`)
    (:`Right`
      (if _returnvalue
        (set `self.SpriteRotationFloat` 0.0)
        (else
          (set `self.SpriteRotationFloat` 180.0))))
    (:`Forward`
      (if (> (.y InVec) (.y (`SceneComponent.K2_GetComponentLocation` (`self.CapsuleComponent`))))
        (set `self.SpriteRotationFloat` 0.0)
        (else
          (set `self.SpriteRotationFloat` 180.0))))
    (:`Left`
      (if (not _returnvalue)
        (set `self.SpriteRotationFloat` 0.0)
        (else
          (set `self.SpriteRotationFloat` 180.0)))))
  (`SceneComponent.K2_SetRelativeRotation` (`self.Sprite`) (`KismetMathLibrary.MakeRotator` 0.0 0.0 (`self.SpriteRotationFloat`)) false false))

(fn `MouseLineTrace`
  (returns (OutHit :type "HitResult Structure"))
  (bind (_worldlocation _worlddirection) (`PlayerController.DeprojectMousePositionToWorld` (`GameplayStatics.GetPlayerController` 0)))
  (bind _outhit (`KismetSystemLibrary.LineTraceSingleForObjects` :`Start` _worldlocation :`End` (+ _worldlocation (* _worlddirection 2000.0)) :`ObjectTypes` (`self.Object TypesForLineTrace`) :`DrawDebugType` "ForDuration" :`bIgnoreSelf` false :`TraceColor` (struct :`G` 0.039124 :`B` 1.0 :`A` 0.188)))
  (return _outhit))

(fn `UserConstructionScript`)